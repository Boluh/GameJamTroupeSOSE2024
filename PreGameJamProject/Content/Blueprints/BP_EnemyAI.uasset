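; Zombie enemy that walks toward a fixed map point until pawn sensing spots something, then chases and attacks the player.
; On reaching the player, it deals randomized damage and plays an attack montage, whose length gates the next hit.
; TakeDmg subtracts randomized projectile damage from HP, while Tick watches for zero HP to play the death montage and destroy the actor.
; An older projectile-hit chain is left unconnected.
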(event OnSeePawn(PawnSensing)
  (params (Pawn :type Pawn%20Object%20Reference))
  (Variables|Default|SetisSeeingPlayer true)
  (CallFunction|FollowPlayer))

(event Custom|FollowPlayer
  (if (Variables|Default|GetisSeeingPlayer)
    (AI|AIMoveTo self "0, 0, 0" (Game|GetPlayerCharacter 0) 5.0 false
      (:OnSuccess
        (if (Variables|Default|GetcanAttack)
          (Game|Damage|ApplyDamage (Game|GetPlayerCharacter 0) (* (Variables|Default|GetDamage) (Math|Random|RandomFloatinRange 0.7 1.3)) 0 0)
          (Variables|Default|SetcanAttack false)
          ;[0 0 0] Hier fehlt ne Animation
          (bind _returnvalue (Animation|PlayAnimMontage "/Game/Animations/Zombie/AnimMonZombieAttk.AnimMonZombieAttk" 2.0 "None"))
          (Utilities|FlowControl|Delay _returnvalue)
          (Variables|Default|SetcanAttack true))))
    (else
      (Variables|Default|SetisSeeingPlayer false))))

(event EventBeginPlay
  (if (not (Variables|Default|GetisSeeingPlayer))
    (AI|AIMoveTo self (Math|Vector|MakeVector 3.5e+04 3.5e+04 0.0) 0 5.0 false
      (:OnSuccess
        (Components|Movement|StopMovementImmediately (Variables|Character|GetCharacterMovement))))))

(event Collision|EventActorBeginOverlap
  (params (OtherActor :type Actor%20Object%20Reference)))

(event EventTick
  (params (DeltaSeconds :type Float%20%28single-precision%29))
  (if (<= (Variables|Default|GetHP) 0.0)
    (Components|Movement|StopMovementImmediately (Variables|Character|GetCharacterMovement))
    (bind _returnvalue (Animation|PlayAnimMontage "/Game/Animations/Zombie/AnimMonZombieDeath.AnimMonZombieDeath" 1.0 "None"))
    (Variables|Default|SetisDead true)
    (Utilities|FlowControl|Delay _returnvalue)
    (Actor|DestroyActor)))

(fn ConstructionScript)

(fn TakeDmg
  (Variables|Default|SetHP (- (Variables|Default|GetHP) (* (Variables|Default|GetProjectileDmg) (Math|Random|RandomFloatinRange 0.7 1.3)))))